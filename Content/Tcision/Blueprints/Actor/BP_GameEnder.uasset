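; BP_GameEnder is a triggerable, multicast actor that ends the game with a given Conclusion, whose title labels it via the construction script.
; Trigger stops the active sequencer from the GameState and moves the player pawn to an end camera position.
; It then puts an end-game widget built from the Conclusion on EndScreen and shows the HUD end screen.
; Finally, it adds its unlocking scenarios to available levels and saves progress.
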(event `self.Trigger`
  (params (TriggererController :type "Controller Object Reference") (Triggerer :type "Object Object Reference") (Tag :type Name) (Payload :type "Object Object Reference"))
  (`|ExecutionSequence`
    (:`then_0`
      (bind _savedvalue (`/LibAmasson/Blueprints/BPL_GenericMacrosExtension.SaveValidObject` (`self.GetComponentByClass` (`GameplayStatics.GetGameState`) "/Game/Tcision/Blueprints/Components/BP_ActiveSequencerReference.BP_ActiveSequencerReference_C"))
        (:`Is Valid`
          (bind _activesequencer (`/Game/Tcision/Blueprints/Components/BP_ActiveSequencerReference.ActiveSequencer` _savedvalue)
            (:`then`
              (`/Game/Tcision/Blueprints/Actor/BP_InteractiveNarrationSequencer.StopSequence` _activesequencer))
            (:`else`)))))
    (:`then_1`
      (bind _endcameraposition (`self.EndCameraPosition`)
        (:`then`
          (`self.K2_SetActorTransform` (`GameplayStatics.GetPlayerPawn` 0) (`self.GetTransform` _endcameraposition) false false))
        (:`else`)))
    (:`then_2`
      (bind _endscreen (`self.EndScreen`)
        (:`then`
          (bind _returnvalue (`|CreateWidget` "/Game/Tcision/Blueprints/UI/Widgets/Scenario/WBP_EndGameScreen.WBP_EndGameScreen_C" null (`self.Conclusion`)))
          (`WidgetComponent.SetWidget` (`/Game/Tcision/Blueprints/Actor/BP_Screen.Widget` _endscreen) _returnvalue))
        (:`else`)))
    (:`then_3`
      (bind _ashud_tcision (cast `/Game/Tcision/Blueprints/UI/HUD_Tcision` (`PlayerController.GetHUD` (`GameplayStatics.GetPlayerController` 0))))
      (`/Game/Tcision/Blueprints/UI/HUD_Tcision.ShowEndGameScreen` _ashud_tcision))
    (:`then_4`
      (`self.UnlockScenarios`))))

(fn `GetTriggerMode`
  (returns (ReturnValue :type "ETriggerMode Enum"))
  (return "TM_Multicast"))

(fn `UnlockScenarios`
  (bind _progressmanager (`/Game/Tcision/Blueprints/Game/GI_TCision.ProgressManager` (`AmassonBlueprintFunctionLibrary.GetGameInstance` null "/Game/Tcision/Blueprints/Game/GI_TCision.GI_TCision_C")))
  (bind _progress (`/Game/Tcision/Blueprints/Object/BP_ProgressionManager.GetProgressObject` _progressmanager))
  (for _array_element (`self.UnlockingScenarios`)
    (`BlueprintSetLibrary.Set_Add` (`/Game/Tcision/Blueprints/Object/SG_TCisionProgress.AvailableLevels` _progress) _array_element))
  (`/Game/Tcision/Blueprints/Object/BP_ProgressionManager.SaveProgress` _progressmanager))

(fn `UserConstructionScript`
  (`TextRenderComponent.K2_SetText` (`self.Name`) (`.Title_6_FDB9BE4AA8B8401DA77E95B980F3A92C` (break `/Game/Tcision/Blueprints/Structures/S_EndGameConclusion` (`self.Conclusion`)))))