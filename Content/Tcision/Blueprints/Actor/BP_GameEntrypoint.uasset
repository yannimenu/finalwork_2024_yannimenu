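; BP_GameEntrypoint is a placeable actor that kicks off a scenario when play begins.
; On BeginPlay it sends a tagged trigger message to its StarterActor, then shows its scenario text through the Tcision HUD.
; Its construction script sets a name label to the scenario text and adds an arrow stretched toward the starter actor as an editor aid, compensating for actor X scale.
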(event `self.ReceiveBeginPlay`
  (message `Triggerable.Trigger` (`self.StarterActor`) null self (`self.StarterTag`) null)
  (bind _ashud_tcision (cast `/Game/Tcision/Blueprints/UI/HUD_Tcision` (`PlayerController.GetHUD` (`GameplayStatics.GetPlayerController` 0))))
  (`/Game/Tcision/Blueprints/UI/HUD_Tcision.ShowScenarioText` _ashud_tcision (`self.ScenarioText`)))

(fn `GenerateEditorHelpers`
  (bind _returnvalue_x (`KismetMathLibrary.BreakVector` (`self.GetActorScale3D`)))
  (bind _returnvalue (`self.K2_GetActorLocation`))
  (bind _starteractor (`self.StarterActor`)
    (:`then`
      (bind _returnvalue_2 (`AddComponent|NODE_AddArrowComponent-0`))
      (bind _returnvalue_3 (`self.K2_GetActorLocation` _starteractor))
      (set `ArrowComponent.ArrowLength` (`KismetMathLibrary.Vector_Distance` _returnvalue_3 _returnvalue) _returnvalue_2)
      (`SceneComponent.K2_SetWorldRotation` _returnvalue_2 (`KismetMathLibrary.FindLookAtRotation` _returnvalue _returnvalue_3) false false)
      (`SceneComponent.SetRelativeScale3D` _returnvalue_2 (`KismetMathLibrary.MakeVector` (/ 1.0 _returnvalue_x) 1.0 1.0)))
    (:`else`)))

(fn `UserConstructionScript`
  (`self.GenerateEditorHelpers`)
  (`TextRenderComponent.K2_SetText` (`self.Name`) (`self.ScenarioText`)))