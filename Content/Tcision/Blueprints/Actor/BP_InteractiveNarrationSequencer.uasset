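; Triggerable sequencer actor for interactive narration, wrapping a level sequence with tag-keyed narration text and player choices.
; Narration and choices display through HUD_Tcision; showing choices pauses the sequence, while finishing or stopping clears narration.
; On trigger or play, it broadcasts a stop to other cinematics via GS_TCision, then registers as the active sequencer.
; Construction draws editor arrows to each choice's target actor and labels it with the sequence name.
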(event `self.ReceiveBeginPlay`
  (`self.AssignSequencePlayerEvents`))

(event `self.Trigger`
  (params (TriggererController :type "Controller Object Reference") (Triggerer :type "Object Object Reference") (Tag :type Name) (Payload :type "Object Object Reference"))
  (`self.SubscribeToGlobalChoiceNotifier`)
  (`parent.Trigger` TriggererController Triggerer Tag Payload))

(event `AssignSequencePlayerEvents`
  (bind _sequenceplayer (`self.SequencePlayer`)
    (:`then`
      (add `MovieSceneSequencePlayer.OnFinished` _sequenceplayer (delegate `OnFinished_Event`))
      (add `MovieSceneSequencePlayer.OnStop` _sequenceplayer (delegate `OnStop_Event`)))
    (:`else`)))

(event `OnFinished_Event`
  (`self.ClearNarrationText` :!label _label))

(event `OnStop_Event`
  (goto _label))

(event `PlaySequence`
  (`self.SubscribeToGlobalChoiceNotifier`)
  (`MovieSceneSequencePlayer.Play` (`self.SequencePlayer`)))

(event `SubscribeToGlobalChoiceNotifier`
  (bind _savedvalue (`/LibAmasson/Blueprints/BPL_GenericMacrosExtension.SaveValidObject` (`AmassonBlueprintFunctionLibrary.GetGameState` null "/Game/Tcision/Blueprints/Game/GS_TCision.GS_TCision_C"))
    (:`Is Valid`
      (`/Game/Tcision/Blueprints/Game/GS_TCision.BroadcastStopAllCinamatics` _savedvalue)
      (add `/Game/Tcision/Blueprints/Game/GS_TCision.StopAllCinematics` _savedvalue (delegate `StopAllCinematics_Event`))
      (set `/Game/Tcision/Blueprints/Components/BP_ActiveSequencerReference.ActiveSequencer` self (`/Game/Tcision/Blueprints/Game/GS_TCision.ActiveSequencerRef` _savedvalue)))))

(event `StopAllCinematics_Event`
  (`self.StopSequence`)
  (`self.ClearNarrationText`)
  (remove `/Game/Tcision/Blueprints/Game/GS_TCision.StopAllCinematics` (stale `SubscribeToGlobalChoiceNotifier` _savedvalue) (delegate `StopAllCinematics_Event`)))

(event `StopSequence`
  (bind _sequenceplayer (`self.SequencePlayer`))
  (if (or (`MovieSceneSequencePlayer.IsPlaying` _sequenceplayer) (`MovieSceneSequencePlayer.IsPaused` _sequenceplayer))
    (`MovieSceneSequencePlayer.Stop` _sequenceplayer)))

(event `PauseSequence`
  (bind _sequenceplayer (`self.SequencePlayer`))
  (if (`MovieSceneSequencePlayer.IsPlaying` _sequenceplayer)
    (`MovieSceneSequencePlayer.Pause` _sequenceplayer)))

(event `ShowCurrentChoiceWidgets`
  (params (ChoiceTag :type Name))
  (bind (_value _returnvalue) (`BlueprintMapLibrary.Map_Find` (`self.ChoiceLists`) ChoiceTag))
  (if _returnvalue
    (bind _ashud_tcision (cast `/Game/Tcision/Blueprints/UI/HUD_Tcision` (`PlayerController.GetHUD` (`GameplayStatics.GetPlayerController` 0))))
    (`/Game/Tcision/Blueprints/UI/HUD_Tcision.ShowChoicePrompt` _ashud_tcision _value self)
    (`self.PauseSequence`)
    (else
      (`KismetSystemLibrary.PrintText` (`|FormatText` self "Invalid request to display choices {choices} sequence {self}" ChoiceTag) true true (struct :`R` 1.0 :`A` 1.0) 5.0))))

(event `ShowNarrationText`
  (params (NarrationTag :type "Name (by ref)"))
  (bind (_value _returnvalue) (`BlueprintMapLibrary.Map_Find` (`self.NarrationList`) NarrationTag))
  (if _returnvalue
    (bind _ashud_tcision (cast `/Game/Tcision/Blueprints/UI/HUD_Tcision` (`PlayerController.GetHUD` (`GameplayStatics.GetPlayerController` 0))))
    (`/Game/Tcision/Blueprints/UI/HUD_Tcision.ShowSitutationText` _ashud_tcision (`.Text_2_8A60DCC05A0D49629A720CB4E0D62782` (break `/Game/Tcision/Blueprints/Structures/S_SituationInfos` _value)) self)
    (else
      (`KismetSystemLibrary.PrintText` (`|FormatText` self "Invalid request to display situation {situation} sequence {self}" NarrationTag) true true (struct :`R` 1.0 :`A` 1.0) 5.0))))

(event `ClearNarrationText`
  (bind _returnvalue (`GameplayStatics.GetPlayerController` 0))
  (`/Engine/EditorBlueprintResources/StandardMacros.IsValid` _returnvalue
    (:`Is Valid`
      (bind _ashud_tcision (cast `/Game/Tcision/Blueprints/UI/HUD_Tcision` (`PlayerController.GetHUD` _returnvalue)))
      (`/Game/Tcision/Blueprints/UI/HUD_Tcision.ClearSituationText` _ashud_tcision self))))

(fn `GenerateEditorHelpers`
  (bind _returnvalue_x (`KismetMathLibrary.BreakVector` (`self.GetActorScale3D`)))
  (bind _returnvalue (`self.K2_GetActorLocation`))
  (`|ExecutionSequence`
    (:`then_0`
      (bind _values (`BlueprintMapLibrary.Map_Values` (`self.ChoiceLists`)))
      (for _array_element _values
        (for _array_element_2 (`.Choices_5_0EFD0F07236847088DE73B38112BA3FC` (break `/Game/Tcision/Blueprints/Structures/S_ChoiceList` _array_element))
          (bind (_text _format _triggering) (break `/Game/Tcision/Blueprints/Structures/S_ActionChoice` _array_element_2))
          (`/Engine/EditorBlueprintResources/StandardMacros.IsValid` _triggering
            (:`Is Valid`
              (bind _returnvalue_2 (`AddComponent|NODE_AddArrowComponent-2`))
              (bind _returnvalue_3 (`self.K2_GetActorLocation` _triggering))
              (set `ArrowComponent.ArrowLength` (`KismetMathLibrary.Vector_Distance` _returnvalue_3 _returnvalue) _returnvalue_2)
              (`SceneComponent.K2_SetWorldRotation` _returnvalue_2 (`KismetMathLibrary.FindLookAtRotation` _returnvalue _returnvalue_3) false false)
              (`SceneComponent.SetRelativeScale3D` _returnvalue_2 (`KismetMathLibrary.MakeVector` (/ 1.0 _returnvalue_x) 1.0 1.0)))))))
    (:`then_1`
      (`TextRenderComponent.K2_SetText` (`self.Name`) (`KismetTextLibrary.Conv_StringToText` (`KismetSystemLibrary.GetObjectName` (`self.LevelSequenceAsset`)))))))

(fn `GetTriggerMode`
  (returns (ReturnValue :type "ETriggerMode Enum"))
  (return "TM_Multicast"))

(fn `UserConstructionScript`
  (`self.GenerateEditorHelpers`))