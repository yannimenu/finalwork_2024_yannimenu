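; Level Sequence Director for TCision that lets sequences drive narration text, choice widgets and pausing in narrative situations.
; Fixed-tag events (NarrativeDefault, NarrativeQuestion, ChoicesDefault) forward to Notify functions for narration and choices.
; Those functions and NotifyFreeze reach the active sequencer through the GS_TCision game state to show content or pause.
; NotifyClearNarration clears text on SituationSequencer without doing that lookup itself.
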(event `NarrativeDefault`
  (`self.NotifyNarration` "Default"))

(event `NarrativeQuestion`
  (`self.NotifyNarration` "Question"))

(event `ChoicesDefault`
  (`self.NotifyChoices` "Default"))

(fn `NotifyChoices`
  (params (ChoiceTag :type Name :default "Default"))
  (`/Game/Tcision/Blueprints/Actor/BP_InteractiveNarrationSequencer.ShowCurrentChoiceWidgets` (`/Game/Tcision/Blueprints/Components/BP_ActiveSequencerReference.ActiveSequencer` (`/Game/Tcision/Blueprints/Game/GS_TCision.ActiveSequencerRef` (`AmassonBlueprintFunctionLibrary.GetGameState` null "/Game/Tcision/Blueprints/Game/GS_TCision.GS_TCision_C"))) ChoiceTag))

(fn `NotifyClearNarration`
  (`/Game/Tcision/Blueprints/Actor/BP_InteractiveNarrationSequencer.ClearNarrationText` (`self.SituationSequencer`)))

(fn `NotifyFreeze`
  (`/Game/Tcision/Blueprints/Actor/BP_InteractiveNarrationSequencer.PauseSequence` (`/Game/Tcision/Blueprints/Components/BP_ActiveSequencerReference.ActiveSequencer` (`/Game/Tcision/Blueprints/Game/GS_TCision.ActiveSequencerRef` (`AmassonBlueprintFunctionLibrary.GetGameState` null "/Game/Tcision/Blueprints/Game/GS_TCision.GS_TCision_C")))))

(fn `NotifyNarration`
  (params (SituationTag :type Name :default "Default"))
  (bind _output_get (set `self.SituationSequencer` (`/Game/Tcision/Blueprints/Components/BP_ActiveSequencerReference.ActiveSequencer` (`/Game/Tcision/Blueprints/Game/GS_TCision.ActiveSequencerRef` (`AmassonBlueprintFunctionLibrary.GetGameState` null "/Game/Tcision/Blueprints/Game/GS_TCision.GS_TCision_C")))))
  (`/Game/Tcision/Blueprints/Actor/BP_InteractiveNarrationSequencer.ShowNarrationText` _output_get SituationTag))