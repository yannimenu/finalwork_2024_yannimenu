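; BP_ProgressionManager loads, holds and saves the game's progress as an SG_TCisionProgress save game object in a single named slot.
; LoadProgress reads the slot, creating a fresh save object when none exists or the cast fails.
; GetProgressObject lazily calls LoadProgress when the cached object is invalid, then returns it.
; SaveProgress writes the cached object back to the slot without checking that it is valid.
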(fn `GetProgressObject`
  (returns (Progress :type "/Game/Tcision/Blueprints/Object/SG_TCisionProgress Object Reference"))
  (`|ExecutionSequence`
    (:`then_0`
      (`/Engine/EditorBlueprintResources/StandardMacros.IsValid` (`self.Progress`)
        (:`Is Not Valid`
          (`self.LoadProgress`))))
    (:`then_1`
      (return (`self.Progress`)))))

(fn `LoadProgress`
  (bind _returnvalue (`GameplayStatics.DoesSaveGameExist` (`self.ProgressSlotName`)))
  (if _returnvalue
    (bind _returnvalue_2 (`GameplayStatics.LoadGameFromSlot` (`self.ProgressSlotName`)))
    (bind _assg_tcision_progress (cast `/Game/Tcision/Blueprints/Object/SG_TCisionProgress` _returnvalue_2)
      (:`then`
        (set `self.Progress` _assg_tcision_progress))
      (:`CastFailed`
        (bind _returnvalue_3 (`GameplayStatics.CreateSaveGameObject` "/Game/Tcision/Blueprints/Object/SG_TCisionProgress.SG_TCisionProgress_C" :!label _label))
        (set `self.Progress` _returnvalue_3)))
    (else
      (goto _label))))

(fn `SaveProgress`
  (`GameplayStatics.SaveGameToSlot` (`self.Progress`) (`self.ProgressSlotName`)))